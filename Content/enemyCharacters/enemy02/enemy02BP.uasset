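; Enemy character Blueprint that takes damage and fires bullets.
; takeDMG subtracts damage from EnemyHP, destroying the actor at zero or below and printing the damage otherwise.
; rootyTootyPointAndShooty spawns a BulletBP at Arrow1's transform, with a DoOnce and Delay acting as a two-second cooldown.
; A disconnected chain that looks up VirusBP actors and calls the shot never runs, and Tick is empty.
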(event `self.ReceiveTick`
  (params (DeltaSeconds :type "Float (single-precision)")))

(event `takeDMG`
  (params (DMGTaken :type Integer))
  (bind _output_get (set `self.enemyHP` (- (`self.enemyHP`) DMGTaken)))
  (if (<= _output_get 0)
    (`self.K2_DestroyActor`)
    (else
      (`KismetSystemLibrary.PrintString` (`KismetStringLibrary.Conv_IntToString` DMGTaken)))))

(event `rootyTootyPointAndShooty`
  (`/Engine/EditorBlueprintResources/StandardMacros.DoOnce` false :!label _label
    (:`Completed`
      (`|SpawnActorFromClass` "/Game/enemyCharacters/enemy02/bulletBP.bulletBP_C" (`SceneComponent.K2_GetComponentToWorld` (`self.Arrow1`)) "Undefined" "OverrideRootScale" null null)
      (`KismetSystemLibrary.Delay` 2.0)
      (goto _label :!via `Reset`))))

(fn `UserConstructionScript`)