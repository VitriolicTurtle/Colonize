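; Enemy 03 Blueprint: a chasing enemy with a health bar widget that can award points to the player's virusBP.
; Tick refreshes the bar and steps one unit per axis toward the player on X and Y, independent of delta time.
; TakeDamage's check looks inverted: it scores and destroys the enemy when health would remain above zero.
; ModifyHealth separately clamps health; the arrow look-at logic is disconnected.
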(event `self.ReceiveTick`
  (params (DeltaSeconds :type "Float (single-precision)"))
  (`|ExecutionSequence`
    (:`then_0`
      (bind _asenemy_health_bar (cast `/Game/enemyUI/enemyHealthBar` (`WidgetComponent.GetUserWidgetObject` (`self.hpbar`))))
      (set `/Game/enemyUI/enemyHealthBar.maxHealth` (`self.enemyMaxHP`) _asenemy_health_bar)
      (set `/Game/enemyUI/enemyHealthBar.currentHealth` (`self.enemyHP`) _asenemy_health_bar)
      (`ProgressBar.SetPercent` (`/Game/enemyUI/enemyHealthBar.ProgressBar_153` _asenemy_health_bar) (/ (`self.enemyHP`) (`self.enemyMaxHP`))))
    (:`then_1`
      (`self.moveToPlayer`)
      (`self.moveToPlayer2`)
      (bind _asbullet_bp (cast `/Game/enemyCharacters/enemy02/bulletBP` (`ActorComponent.GetOwner` (`self.Capsule`))))
      (bind _output_get (set `self.actorref` _asbullet_bp))
      (`PrimitiveComponent.IgnoreActorWhenMoving` (`self.Capsule`) _output_get true))))

(event `moveToPlayer2`
  (bind (_locloc1_x _locloc1_y) (`KismetMathLibrary.BreakVector` (`self.locLoc1`)))
  (bind (_locloc2_x _locloc2_y) (`KismetMathLibrary.BreakVector` (`self.locLoc2`)))
  (bind (_locloc1_x_2 _locloc1_y_2 _locloc1_z) (`KismetMathLibrary.BreakVector` (`self.locLoc1`)))
  (bind (_locloc1_x_3 _locloc1_y_3 _locloc1_z_2) (`KismetMathLibrary.BreakVector` (`self.locLoc1`)))
  (set `self.locLoc1` (`self.K2_GetActorLocation` self))
  (set `self.locLoc2` (`self.K2_GetActorLocation` (`GameplayStatics.GetPlayerCharacter` 0)))
  (if (> _locloc1_y _locloc2_y)
    (`self.K2_SetActorLocation` self (`KismetMathLibrary.MakeVector` _locloc1_x_2 (- _locloc1_y_2 1.0) _locloc1_z) false false)
    (elif (< _locloc1_y _locloc2_y)
      (`self.K2_SetActorLocation` (`KismetMathLibrary.MakeVector` _locloc1_x_3 (+ _locloc1_y_3 1.0) _locloc1_z_2)))))

(event `moveToPlayer`
  (bind _locloc1_x (`KismetMathLibrary.BreakVector` (`self.locLoc1`)))
  (bind _locloc2_x (`KismetMathLibrary.BreakVector` (`self.locLoc2`)))
  (bind (_locloc1_x_2 _locloc1_y _locloc1_z) (`KismetMathLibrary.BreakVector` (`self.locLoc1`)))
  (bind (_locloc1_x_3 _locloc1_y_2 _locloc1_z_2) (`KismetMathLibrary.BreakVector` (`self.locLoc1`)))
  (set `self.locLoc1` (`self.K2_GetActorLocation` self))
  (set `self.locLoc2` (`self.K2_GetActorLocation` (`GameplayStatics.GetPlayerCharacter` 0)))
  (if (> _locloc1_x _locloc2_x)
    (`self.K2_SetActorLocation` self (`KismetMathLibrary.MakeVector` (- _locloc1_x_2 1.0) _locloc1_y _locloc1_z) false false)
    (elif (< _locloc1_x _locloc2_x)
      (`self.K2_SetActorLocation` (`KismetMathLibrary.MakeVector` (+ _locloc1_x_3 1.0) _locloc1_y_2 _locloc1_z_2)))))

(event `takeDamage`
  (params (dmgTaken :type "Float (double-precision)"))
  (bind _returnvalue (- (`self.enemyHP`) dmgTaken))
  (if (<= _returnvalue 0.0)
    (set `self.enemyHP` _returnvalue)
    (else
      (set `self.enemyHP` 0.0)
      (bind _asvirus_bp (cast `/Game/viralCharacter/virusBP` (`GameplayStatics.GetPlayerCharacter` 0)))
      (`/Game/viralCharacter/virusBP.updateScore` _asvirus_bp (`self.points`))
      (`self.K2_DestroyActor`))))

(fn `ModifyHealth`
  (params (`Health to substract` :type "Float (double-precision)"))
  (set `self.enemyHP` (`KismetMathLibrary.FClamp` (- (`self.enemyHP`) `Health to substract`) 0.0 (`self.enemyMaxHP`))))

(fn `UserConstructionScript`)